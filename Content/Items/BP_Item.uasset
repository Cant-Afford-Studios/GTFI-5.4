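; BP_Item is an item Blueprint for the first-person character, with empty UseItem and Reload events that suggest it serves as a base class.
; Attach casts the owner to BP_FirstPersonCharacter and caches it as Player.
; CalculateAim line-traces on Visibility along a given component's forward vector up to Range, returning the hit location or the trace end.
; UseAmmo decrements Ammo when above zero and reports whether it could.
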(event `Attach`
  (bind _asbp_first_person_character (cast `/Game/FirstPerson/Blueprints/BP_FirstPersonCharacter` (`self.GetOwner`)))
  (set `self.Player` _asbp_first_person_character))

(event `Use Item`)

(event `Reload`)

(fn `Calculate Aim`
  (params (Start :type "SceneComponent Object Reference"))
  (returns (AimLocation :type "Vector Structure"))
  (bind _returnvalue (`self.K2_GetComponentLocation` Start))
  (bind _returnvalue_2 (+ _returnvalue (* (`self.GetForwardVector` Start) (`self.Range`))))
  (bind (_outhit _returnvalue_3) (`KismetSystemLibrary.LineTraceSingle` _returnvalue _returnvalue_2 "TraceTypeQuery1"))
  (if _returnvalue_3
    (return (`.Location` (`GameplayStatics.BreakHitResult` _outhit)))
    (else
      (return _returnvalue_2))))

(fn `Use Ammo`
  (returns (Success :type Boolean))
  (locals (CanUse :type Boolean))
  (bind _ammo (`self.Ammo`))
  (bind _output_get (set `local.CanUse` (> _ammo 0)))
  (if _output_get
    (set `self.Ammo` (- _ammo 1)))
  (return (`local.CanUse`)))