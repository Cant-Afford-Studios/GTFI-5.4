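; BP_Grenade is a usable item that throws a grenade projectile from the player's first-person view.
; UseItem passes a DoOnce gate, spends ammo, then spawns BP_GrenadeProjectile at the Muzzle socket, rotated toward the camera aim point plus an offset.
; It plays a pickup sound and rifle shoot montage, then reopens the gate after UseInterval.
; CallConsumed fires when ammo runs out or cannot be used.
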(event `self.Use Item`
  (bind _returnvalue_location (`KismetMathLibrary.BreakTransform` (`self.GetSocketTransform` "Muzzle")))
  ;[1 1 1] Fire Gun
  (`/Engine/EditorBlueprintResources/StandardMacros.DoOnce` false :!label _label
    (:`Completed`
      (bind _success (`self.Use Ammo`))
      (if _success
        (bind _aimlocation (`self.Calculate Aim` (`/Game/FirstPerson/Blueprints/BP_FirstPersonCharacter.FirstPersonCamera` (`self.Player`))))
        (`|SpawnActorFromClass` "/Game/Items/Grenade/BP_GrenadeProjectile.BP_GrenadeProjectile_C" (`KismetMathLibrary.MakeTransform` _returnvalue_location (`KismetMathLibrary.ComposeRotators` (`self.RotationOffset`) (`KismetMathLibrary.FindLookAtRotation` _returnvalue_location _aimlocation))) "Undefined" "OverrideRootScale" null (`self.Player`))
        (`GameplayStatics.PlaySoundAtLocation` "/Engine/VREditor/Sounds/UI/Object_PickUp.Object_PickUp" _returnvalue_location (struct) 1.0 1.0 0.0 null null null null)
        (`AnimInstance.Montage_Play` (`self.GetAnimInstance` (`/Game/FirstPerson/Blueprints/BP_FirstPersonCharacter.FirstPersonMesh` (`self.Player`))) "/Game/FirstPersonArms/Animations/FP_Rifle_Shoot_Montage.FP_Rifle_Shoot_Montage" 1.0 "MontageLength" 0.0 true)
        (`KismetSystemLibrary.Delay` (`self.UseInterval`))
        (`self.Reset Use`)
        (if (<= (`self.Ammo`) 0)
          (`self.Consumed`))
        (else
          (`self.Consumed`))))))

(event `Reset Use`
  ;[1 1 1] Fire Gun
  (goto _label :!via `Reset`))