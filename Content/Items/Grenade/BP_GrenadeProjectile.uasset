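; BP_GrenadeProjectile is a grenade projectile that explodes on its first hit and then destroys itself.
; The hit applies falloff radial damage at full strength within half the explosion radius, tapering out to the full radius.
; A sphere overlap at the impact point finds nearby components and gives physics-simulating ones a linear-falloff radial impulse.
; Debug spheres briefly draw both damage radii.
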(event `self.ReceiveHit`
  (params (MyComp :type "PrimitiveComponent Object Reference") (Other :type "Actor Object Reference") (OtherComp :type "PrimitiveComponent Object Reference") (bSelfMoved :type Boolean) (HitLocation :type "Vector Structure") (HitNormal :type "Vector Structure") (NormalImpulse :type "Vector Structure") (Hit :type "HitResult Structure (by ref)"))
  (bind _explosionradius (`self.ExplosionRadius`))
  (bind _impulsestrength (`self.ImpulseStrength`))
  (bind _explosionradius_2 (`self.ExplosionRadius`))
  ;[0.05035 0.05035 0.05035] Explode On Hit
  (`GameplayStatics.ApplyRadialDamageWithFalloff` :`BaseDamage` (`self.Damage`) :`MinimumDamage` 1.0 :`Origin` HitLocation :`DamageInnerRadius` (/ _explosionradius_2 2.0) :`DamageOuterRadius` _explosionradius_2 :`DamageFalloff` 1.0 :`DamageCauser` null :`InstigatedByController` null)
  (`KismetSystemLibrary.DrawDebugSphere` HitLocation (/ _explosionradius 2.0) 12 (struct :`R` 1.0 :`G` 1.0 :`B` 1.0 :`A` 1.0) 0.5 1.0)
  (`KismetSystemLibrary.DrawDebugSphere` HitLocation _explosionradius 12 (struct :`R` 1.0 :`G` 1.0 :`B` 1.0 :`A` 1.0) 0.5 1.0)
  (bind _outcomponents (`KismetSystemLibrary.SphereOverlapComponents` HitLocation (`self.ExplosionRadius`) (`self.ImpulseObjectTypes`) null (`|MakeArray` self :!type "Actor Object Reference")))
  (for _array_element _outcomponents
    (if (`SceneComponent.IsSimulatingPhysics` _array_element "None")
      (`PhysicsObjectBlueprintLibrary.ApplyRadialImpulse` _array_element HitLocation (`self.ExplosionRadius`) _impulsestrength "RIF_Linear" false 0.0 false 0.0 _impulsestrength)))
  (`self.K2_DestroyActor`))

(fn `UserConstructionScript`
  (`parent.UserConstructionScript`))