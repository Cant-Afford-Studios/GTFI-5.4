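; Base enemy Blueprint that handles health, damage stats and death, scaled by the difficulty level from BP_FirstPersonGameMode.
; At BeginPlay it scales health and damage exponentially by level, then binds to difficulty level-up, which updates only damage, leaving health at its spawn scaling.
; Incoming damage lowers health and plays an attached hit sound, or triggers death below zero.
; Death notifies the game mode, unpossesses the controller and destroys the actor after a short delay.
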(event `self.ReceiveBeginPlay`
  (bind _asbp_first_person_game_mode (cast `/Game/FirstPerson/Blueprints/BP_FirstPersonGameMode` (`GameplayStatics.GetGameMode`)))
  (bind _output_get (set `self.GameMode` _asbp_first_person_game_mode))
  ;[1 1 1] Set Stats Based on Spawned Difficulty
  (bind _level (`/Game/FirstPerson/Blueprints/BP_FirstPersonGameMode.Get Level` _output_get))
  (set `self.CurrentHealth` (* (`KismetMathLibrary.MultiplyMultiply_FloatFloat` (`self.HealthLevelMult`) (`KismetMathLibrary.Conv_IntToDouble` _level)) (`self.Health`)))
  (`self.Set Damage Level` _level)
  (add `/Game/FirstPerson/Blueprints/BP_FirstPersonGameMode.DifficultyLevelUp` (`self.GameMode`) (delegate `Set Damage Level`)))

(event `Set Damage Level`
  (params (Level :type Integer))
  ;[1 1 1] Set Damaged Based on Level
  (set `self.CurrentDamage` (* (`self.Damage`) (`KismetMathLibrary.MultiplyMultiply_FloatFloat` (`self.DamageLevelMult`) (`KismetMathLibrary.Conv_IntToDouble` Level)))))

(event `self.ReceiveAnyDamage`
  (params (Damage :type "Float (single-precision)") (DamageType :type "DamageType Object Reference") (InstigatedBy :type "Controller Object Reference") (DamageCauser :type "Actor Object Reference"))
  ;[1 1 1] Take Damage
  (bind _output_get (set `self.CurrentHealth` (- (`self.CurrentHealth`) Damage)))
  (if (< _output_get 0.0)
    (`self.Die` DamageCauser)
    (else
      (`GameplayStatics.SpawnSoundAttached` (`self.DamageSound`) (`self.CapsuleComponent`) "None" (0.0 0.0 0.0) (struct) "KeepRelativeOffset" false 1.0 1.0 0.0 null null))))

(event `Die`
  (params (Killer :type "Actor Object Reference"))
  ;[1 1 1] Death
  (`/Game/FirstPerson/Blueprints/BP_FirstPersonGameMode.RemoveEnemy` (`self.GameMode`))
  (`Controller.UnPossess` (`self.GetController`))
  (`KismetSystemLibrary.Delay` 0.5)
  (`self.K2_DestroyActor`))

(fn `UserConstructionScript`)