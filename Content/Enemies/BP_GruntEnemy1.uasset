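; BP_GruntEnemy1 is a grunt enemy Blueprint that passes detected player positions to its AI.
; When notified of an enemy detection, it writes the player's current location into the blackboard's TargetLocation key as a one-time snapshot.
; BeginPlay, overlap and Tick are disabled stubs, and the construction script only calls its parent.
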(event `/Game/Enemies/BPI_AI.NotifyEnemyDetected`
  (params (Player :type "Character Object Reference"))
  (`BlackboardComponent.SetValueAsVector` (`AIBlueprintHelperLibrary.GetBlackboard` null) "TargetLocation" (`self.K2_GetActorLocation` Player)))

(fn `UserConstructionScript`
  (`parent.UserConstructionScript`))